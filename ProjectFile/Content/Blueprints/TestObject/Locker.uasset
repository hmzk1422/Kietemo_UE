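; Test locker actor whose door the player character opens and closes by interacting with it.
; Area's begin overlap sets an Overlap flag, which nothing clears.
; Tick casts the overlapping actor to CharacterBP and, throttled by a DoOnce reset after a short delay, passes Overlap and Interact to OpenClose.
; OpenClose alternates the opening and closing animations through DoorOpen; a delayed WhileLoop macro is defined but unused.
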(event `self.ReceiveTick`
  (params (DeltaSeconds :type "Float (single-precision)"))
  (bind _ascharacter_bp (cast `/Game/Blueprints/Character/CharacterBP` (stale `self.Area.OnComponentBeginOverlap` OtherActor)))
  (`/Engine/EditorBlueprintResources/StandardMacros.DoOnce` false :!label _label
    (:`Completed`
      (`self.OpenClose` (and (stale `self.Area.OnComponentBeginOverlap` _output_get) (`/Game/Blueprints/Character/CharacterBP.Interact` _ascharacter_bp)))
      (`KismetSystemLibrary.RetriggerableDelay` 0.25)
      (goto _label :!via `Reset`))))

(event `self.Area.OnComponentBeginOverlap`
  (params (OverlappedComponent :type "PrimitiveComponent Object Reference") (OtherActor :type "Actor Object Reference") (OtherComp :type "PrimitiveComponent Object Reference") (OtherBodyIndex :type Integer) (bFromSweep :type Boolean) (SweepResult :type "HitResult Structure (by ref)"))
  (bind _output_get (set `self.Overlap` true)))

(event `OpenClose`
  (params (Condition :type Boolean))
  (bind _locker (`self.Locker`))
  (if Condition
    (if (`self.DoorOpen`)
      (`SkeletalMeshComponent.PlayAnimation` _locker "/Game/StandardContent/Meshes/structures/Prop/Locker/LockerOpen.LockerOpen" false)
      (set `self.DoorOpen` false)
      (else
        (`SkeletalMeshComponent.PlayAnimation` _locker "/Game/StandardContent/Meshes/structures/Prop/Locker/LockerClosing.LockerClosing" false)
        (set `self.DoorOpen` true)))))

(fn `UserConstructionScript`)