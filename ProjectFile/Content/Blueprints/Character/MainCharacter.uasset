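; Main character Blueprint for melee combat with katana, staff or fists.
; Number keys identify slotted weapons by display name through a delayed-loop macro and toggle drawing them, while Tick maps CurrentTool to attack montages and block resistance.
; Fist hits use a looping timer that line-traces between hand sockets.
; Incoming damage handles block reduction, random timed crippling, knockback and death; regeneration and the damage-gate reset are unconnected.
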(event `IdentifyTool`
  ;[0 0 0] Identify Tool
  (`|ExecutionSequence`
    (:`then_0`
      (bind _classification (`self.TestTool` (`self.IsKatana`) (`self.KatanaMax`) (`self.KatanaIdentify`) (`self.Weapon`))
        (:`Completed`
          (set `self.IsKatana` _classification))))
    (:`then_1`
      (bind _classification_2 (`self.TestTool` (`self.IsStaff`) (`self.StaffMax`) (`self.StaffIdentify`) (`self.Weapon2`))
        (:`Completed`
          (set `self.IsStaff` _classification_2))))))

(event `InputAction|Attack`
  (params (Key :type "Key Structure"))
  ;[0 0 0] Identify Tool
  ;;[1 1 1] Attacks
  (:`Pressed`
    (`self.DoAttack` Key)))

(event `Key|One`
  (params (Key :type "Key Structure"))
  ;[0 0 0] Identify Tool
  ;;[1 1 1] Attacks
  (:`Pressed`
    (`self.IdentifyTool`)
    (if (`self.Katana_Unequip`)
      (`self.DrawSword`)
      (else
        (`self.DrawSword`)
        (`self.UnarmedMode`)))))

(event `Key|Two`
  (params (Key :type "Key Structure"))
  ;[0 0 0] Identify Tool
  ;;[1 1 1] Attacks
  (:`Pressed`
    (`self.IdentifyTool`)
    (if (`self.Staff_Unequip`)
      (`self.DrawStaff`)
      (else
        (`self.DrawStaff`)
        (`self.UnarmedMode`)))))

(event `Key|G`
  (params (Key :type "Key Structure"))
  ;[0 0 0] Identify Tool
  ;;[1 1 1] Attacks
  (:`Pressed`
    (`self.BlockEvent`))
  (:`Released`
    (`self.ReleaseBlockEvent`)))

(event `TriggerFist`
  ;[0 0 0] DamageApplyStart
  (bind _returnvalue (`KismetSystemLibrary.K2_SetTimerDelegate` (delegate `FistLineTrace`) 0.05 true))
  (set `self.TriggerFistEvent` _returnvalue))

(event `StaffMode`
  ;[0 0 0] Mode
  (`|ExecutionSequence`
    (:`then_0`
      (set `self.BottomAttackAnim` null))
    (:`then_1`
      (set `self.MainAttackAnim` "/Game/StandardContent/Meshes/Character/Main_character/Main_CharacterAnim/Combat/Staff/MaleStMainAttackM.MaleStMainAttackM"))
    (:`then_2`
      (set `self.UpperAttackAnim` null))
    (:`then_3`
      (set `self.BlockAnim` null))
    (:`then_4`
      (`|ExecutionSequence`
        (:`then_0`
          (set `self.BlockResistance` 0.6))
        (:`then_1`
          (set `self.Weight` 10.0))))))

(event `FistLineTrace`
  (bind _mesh (`self.Mesh`))
  ;[0 0 0] DamageApplyStart
  (bind _outhit (`KismetSystemLibrary.LineTraceSingle` :`Start` (`SceneComponent.GetSocketLocation` _mesh "RightHandCSocket") :`End` (`SceneComponent.GetSocketLocation` _mesh "RightSlotLocation") :`TraceChannel` "TraceTypeQuery2" :`DrawDebugType` "ForDuration"))
  (`GameplayStatics.ApplyDamage` (`.HitActor` (`GameplayStatics.BreakHitResult` _outhit)) (`self.FistDamage`)))

(event `UnarmedMode`
  ;[0 0 0] Mode
  (`|ExecutionSequence`
    (:`then_0`
      (set `self.BottomAttackAnim` null))
    (:`then_1`
      (set `self.MainAttackAnim` "/Game/StandardContent/Meshes/Character/Main_character/Main_CharacterAnim/Combat/Fist/MalePunchM.MalePunchM"))
    (:`then_2`
      (set `self.UpperAttackAnim` null))
    (:`then_3`
      (set `self.BlockAnim` null))
    (:`then_4`
      (`|ExecutionSequence`
        (:`then_0`
          (set `self.BlockResistance` 0.3))))))

(event `StopTriggerFist`
  ;[0 0 0] DamageApplyEnd
  (`KismetSystemLibrary.K2_ClearAndInvalidateTimerHandle` (`self.TriggerFistEvent`)))

(event `KatanaMode`
  ;[0 0 0] Mode
  (`|ExecutionSequence`
    (:`then_0`
      (set `self.BottomAttackAnim` "/Game/StandardContent/Meshes/Character/Main_character/Main_CharacterAnim/Combat/Katana/Attacks/KRightAttackM.KRightAttackM"))
    (:`then_1`
      (set `self.MainAttackAnim` "/Game/StandardContent/Meshes/Character/Main_character/Main_CharacterAnim/Combat/Katana/Attacks/KLightAttackM.KLightAttackM"))
    (:`then_2`
      (set `self.UpperAttackAnim` "/Game/StandardContent/Meshes/Character/Main_character/Main_CharacterAnim/Combat/Katana/Attacks/KLeftAttackM.KLeftAttackM"))
    (:`then_3`
      (set `self.BlockAnim` "/Game/StandardContent/Meshes/Character/Main_character/Main_CharacterAnim/Combat/Katana/Defense/MaleKBlockM.MaleKBlockM"))
    (:`then_4`
      (`|ExecutionSequence`
        (:`then_0`
          (set `self.BlockResistance` 0.5))))))

(event `self.ReceiveTick`
  (params (DeltaSeconds :type "Float (single-precision)"))
  (bind _currenttool (`self.CurrentTool`))
  (if (`KismetStringLibrary.EqualEqual_StrStr` _currenttool "Katana")
    (`self.KatanaMode`)
    (elif (`KismetStringLibrary.EqualEqual_StrStr` _currenttool "Staff")
      (`self.StaffMode`)
      (elif (`KismetStringLibrary.EqualEqual_StrStr` _currenttool)
        (`self.UnarmedMode`)))))

(fn `UserConstructionScript`
  (`parent.UserConstructionScript`))