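; Player character Blueprint handling movement, camera, crouching and melee combat with katana and staff draw/sheathe.
; Three montage-driven attacks use DoOnce gates and montage-length delays, and blocking replays its montage while held.
; AnyDamage feeds the EventDamage macro, which applies block reduction, a random block-disabling cripple, hit reaction, knockback, death and delayed health regeneration.
; A custom WhileLoopDelay macro drives the timed loops for block, regeneration, death and stamina.
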(event `self.ReceiveAnyDamage`
  (params (Damage :type "Float (single-precision)") (DamageType :type "DamageType Object Reference") (InstigatedBy :type "Controller Object Reference") (DamageCauser :type "Actor Object Reference"))
  ;[0.5 0.5 0.5 1 30] CharacterStats
  ;;[0 0 0] HP
  (set `self.Hit` true)
  (`self.EventDamage` Damage DamageCauser
    (:`  `
      (set `self.Attacker` DamageCauser)
      (set `self.Agro` true)
      (`KismetSystemLibrary.RetriggerableDelay` 0.2)
      (set `self.Hit` false))))

(event `Key|E`
  (params (Key :type "Key Structure"))
  ;[1 1 1 1 30] katana
  ;;[0 0 0] KeySets
  (:`Pressed`
    (set `self.Interact` true))
  (:`Released`
    (set `self.Interact` false)))

(event `BlockEvent`
  ;[1 1 1 1 30] katana
  ;;[0 0 0] Controls
  ;;;[0 0 0] Block
  (if (not (`self.Crippled`))
    (set `self.Block` true)
    (`self.WhileLoopDelay` (`self.Block`) 0.5
      (:`LoopBody`
        (`self.PlayAnimMontage` (`self.BlockAnim`)))
      (:`Completed`
        (`KismetSystemLibrary.Delay` 2.0)))))

(event `ReleaseBlockEvent`
  ;[1 1 1 1 30] katana
  ;;[0 0 0] Controls
  ;;;[0 0 0] Block
  (set `self.Block` false)
  (`self.StopAnimMontage` (`self.BlockAnim`)))

(event `MainAttack`
  ;[1 1 1 1 30] katana
  ;;[0 0 0] Controls
  ;;;[0 0 0] Attack
  (`/Engine/EditorBlueprintResources/StandardMacros.DoOnce` false :!label _label
    (:`Completed`
      (bind _returnvalue (`self.PlayAnimMontage` (`self.MainAttackAnim`)))
      (`KismetSystemLibrary.RetriggerableDelay` _returnvalue)
      (goto _label :!via `Reset`))))

(event `DoAttack`
  (params (Pressed :type "Key Structure" :default "None"))
  ;[1 1 1 1 30] katana
  ;;[0 0 0] Controls
  ;;;[0 0 0] Attack
  (if (== Pressed "LeftMouseButton")
    (`self.MainAttack`)
    (elif (== Pressed "RightMouseButton")
      (`self.BottomAttack`)
      (elif (== Pressed "MiddleMouseButton")
        (`self.UpperAttack`)))))

(event `UpperAttack`
  ;[1 1 1 1 30] katana
  ;;[0 0 0] Controls
  ;;;[0 0 0] Attack
  (`/Engine/EditorBlueprintResources/StandardMacros.DoOnce` false :!label _label_2
    (:`Completed`
      (bind _returnvalue (`self.PlayAnimMontage` (`self.UpperAttackAnim`)))
      (`KismetSystemLibrary.RetriggerableDelay` _returnvalue)
      (goto _label_2 :!via `Reset`))))

(event `BottomAttack`
  ;[1 1 1 1 30] katana
  ;;[0 0 0] Controls
  ;;;[0 0 0] Attack
  (`/Engine/EditorBlueprintResources/StandardMacros.DoOnce` false :!label _label_3
    (:`Completed`
      (bind _returnvalue (`self.PlayAnimMontage` (`self.BottomAttackAnim`)))
      (`KismetSystemLibrary.RetriggerableDelay` _returnvalue)
      (goto _label_3 :!via `Reset`))))

(event `DrawSword`
  (bind _charactermovement (`self.CharacterMovement`))
  (bind _currenttool (`self.CurrentTool`))
  ;[1 1 1 1 30] katana
  ;;[0 0 0] Sheath/Unsheath
  (if (or (`KismetStringLibrary.EqualEqual_StrStr` _currenttool) (`KismetStringLibrary.EqualEqual_StrStr` _currenttool "Katana"))
    (if (`self.IsKatana`)
      (if (`self.Katana_Unequip`)
        (bind _returnvalue (`self.PlayAnimMontage` "/Game/StandardContent/Meshes/Character/Main_character/Main_CharacterAnim/Combat/Katana/Sheathing/MaleKUnsheathM.MaleKUnsheathM"))
        (set `CharacterMovementComponent.MaxWalkSpeed` 100.0 _charactermovement)
        (`KismetSystemLibrary.Delay` _returnvalue)
        (set `CharacterMovementComponent.MaxWalkSpeed` 150.0 _charactermovement)
        (set `self.CurrentTool` "Katana")
        (else
          (bind _returnvalue_2 (`self.PlayAnimMontage` "/Game/StandardContent/Meshes/Character/Main_character/Main_CharacterAnim/Combat/Katana/Sheathing/MaleKSheathM.MaleKSheathM"))
          (set `CharacterMovementComponent.MaxWalkSpeed` 100.0 _charactermovement)
          (`KismetSystemLibrary.Delay` _returnvalue_2)
          (set `CharacterMovementComponent.MaxWalkSpeed` 150.0 _charactermovement)
          (set `self.CurrentTool` "None"))))))

(event `Key|F`
  (params (Key :type "Key Structure"))
  (:`Pressed`
    (`KismetSystemLibrary.PrintString` (`KismetStringLibrary.Conv_DoubleToString` (`self.Health`)))))

(event `DrawStaff`
  (bind _currenttool (`self.CurrentTool`))
  (bind _charactermovement (`self.CharacterMovement`))
  ;[1 1 1 1 30] katana
  ;;[0 0 0] Sheath/Unsheath
  (if (or (`KismetStringLibrary.EqualEqual_StrStr` _currenttool) (`KismetStringLibrary.EqualEqual_StrStr` _currenttool "Staff"))
    (if (`self.IsStaff`)
      (if (`self.Staff_Unequip`)
        (bind _returnvalue (`self.PlayAnimMontage` "/Game/StandardContent/Meshes/Character/Main_character/Main_CharacterAnim/Combat/Staff/Sheathing/MaleStDrawM.MaleStDrawM"))
        (set `CharacterMovementComponent.MaxWalkSpeed` 100.0 _charactermovement)
        (`KismetSystemLibrary.Delay` _returnvalue)
        (set `CharacterMovementComponent.MaxWalkSpeed` 150.0 _charactermovement)
        (set `self.CurrentTool` "Staff")
        (else
          (bind _returnvalue_2 (`self.PlayAnimMontage` "/Game/StandardContent/Meshes/Character/Main_character/Main_CharacterAnim/Combat/Staff/Sheathing/MaleStSheathM.MaleStSheathM"))
          (set `CharacterMovementComponent.MaxWalkSpeed` 100.0 _charactermovement)
          (`KismetSystemLibrary.Delay` _returnvalue_2)
          (set `CharacterMovementComponent.MaxWalkSpeed` 150.0 _charactermovement)
          (set `self.CurrentTool` "None"))))))

(event `InputAxis|Movement_controls`
  (params (AxisValue :type "Float (single-precision)"))
  ;[0.5 0.5 0.5 1 40] BasicAction
  ;;[0 0 0] Basic movement
  (`self.AddMovementInput` (`self.GetActorForwardVector`) AxisValue))

(event `InputAction|Jump`
  (params (Key :type "Key Structure"))
  ;[0.5 0.5 0.5 1 40] BasicAction
  ;;[0 0 0] Actions
  (:`Pressed`
    (set `self.JumpHeight` (`self.JumpHeight`))
    (`self.Jump`))
  (:`Released`
    (`self.StopJumping`)))

(event `InputAxis|Left_Right`
  (params (AxisValue :type "Float (single-precision)"))
  ;[0.5 0.5 0.5 1 40] BasicAction
  ;;[0 0 0] Basic movement
  (`self.AddMovementInput` (`self.GetActorRightVector`) AxisValue))

(event `InputAction|Run`
  (params (Key :type "Key Structure"))
  (bind _charactermovement (`self.CharacterMovement`))
  ;[0.5 0.5 0.5 1 40] BasicAction
  ;;[0 0 0] Actions
  (:`Pressed`
    (set `CharacterMovementComponent.MaxWalkSpeed` (`self.RunSpeed`) _charactermovement))
  (:`Released`
    (set `CharacterMovementComponent.MaxWalkSpeed` (`self.WalkSpeed`) _charactermovement)))

(event `InputAxis|Rotate_Left_right`
  (params (AxisValue :type "Float (single-precision)"))
  ;[0.5 0.5 0.5 1 40] BasicAction
  ;;[0 0 0] Camera
  (`self.AddControllerYawInput` AxisValue))

(event `InputAction|Crouch`
  (params (Key :type "Key Structure"))
  ;[0.5 0.5 0.5 1 40] BasicAction
  ;;[0 0 0] Actions
  (:`Pressed`
    (if (`self.Crouching`)
      (bind _returnvalue (`self.PlayAnimMontage` "/Game/StandardContent/Meshes/Character/Main_character/Main_CharacterAnim/Movement/Crouch/MaleUncrouchedM.MaleUncrouchedM"))
      (`KismetSystemLibrary.RetriggerableDelay` _returnvalue)
      (`self.UnCrouch`)
      (else
        (set `CharacterMovementComponent.MaxWalkSpeedCrouched` (`self.CrouchSpeed`) (`self.CharacterMovement`))
        (bind _returnvalue_2 (`self.PlayAnimMontage` "/Game/StandardContent/Meshes/Character/Main_character/Main_CharacterAnim/Movement/Crouch/MaleToCrouchM.MaleToCrouchM"))
        (`KismetSystemLibrary.RetriggerableDelay` _returnvalue_2)
        (`self.Crouch`)))))

(event `InputAxis|Rotate_Up_down`
  (params (AxisValue :type "Float (single-precision)"))
  ;[0.5 0.5 0.5 1 40] BasicAction
  ;;[0 0 0] Camera
  (`self.AddControllerPitchInput` AxisValue))

(event `Death`
  ;[1 1 1] Stats
  ;;[0 0 0] Death
  (`self.WhileLoopDelay` (`self.Dead`) (stale _returnvalue)
    (:`LoopBody`
      (bind _returnvalue (`self.PlayAnimMontage` "/Game/StandardContent/Meshes/Character/Main_character/Main_CharacterAnim/Combat/Damaged/MaleDeathM.MaleDeathM")))))

(event `StaminaEventTime`
  (params (Usage :type "Float (double-precision)") (Executing :type Boolean))
  ;[1 1 1] Stats
  (`self.WhileLoopDelay` Executing 1.0
    (:`LoopBody`
      (set `self.Stamina` (- Usage (`self.Stamina`))))))

(fn `UserConstructionScript`)